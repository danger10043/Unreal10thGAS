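; Player character Blueprint that flashes its mesh material, named as a full-charge cue.
; On BeginPlay it creates a dynamic material instance from the mesh's first material slot and caches it.
; The PlayFullChargeFlash event restarts a timeline whose track feeds SetChargeFlashAmount, which writes the ChargeFlashAmount scalar parameter on that instance.
; Nothing in this Blueprint calls the flash event.
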(event `self.ReceiveBeginPlay`
  (bind _returnvalue (`PrimitiveComponent.CreateDynamicMaterialInstance` (`self.Mesh`) 0 null "None"))
  (`/Engine/EditorBlueprintResources/StandardMacros.IsValid` _returnvalue
    (:`Is Valid`
      (set `self.ChargeFlashMaterials` _returnvalue))))

(event `self.PlayFullChargeFlash`
  (bind (_direction `_새_트랙_0`) (`Timeline|TL_FlashTimeline` :!via `PlayFromStart`)
    (:`Update`
      (`self.SetChargeFlashAmount` `_새_트랙_0`))))

(fn `SetChargeFlashAmount`
  (params (Amount :type "Float (double-precision)"))
  (bind _chargeflashmaterials (`self.ChargeFlashMaterials`))
  (`/Engine/EditorBlueprintResources/StandardMacros.IsValid` _chargeflashmaterials
    (:`Is Valid`
      (`MaterialInstanceDynamic.SetScalarParameterValue` _chargeflashmaterials "ChargeFlashAmount" Amount))))

(fn `UserConstructionScript`)